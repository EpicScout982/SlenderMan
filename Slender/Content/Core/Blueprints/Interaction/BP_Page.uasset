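; BP_Page is a collectible page that stays inactive until SeeMe! makes its paper visible and enables it.
; Interacting plays a grab sound, increments PagesCollected on BP_Player, calls PageUpdate and destroys the page.
; When the player enters its box with WeSeePage set, the page's own flashlight replaces the player's flashlight model and light.
; Paired DoOnce gates re-arm each other so leaving the box restores the player's flashlight.
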(event `SeeMe!`
  (`SceneComponent.SetVisibility` (`self.Paper`) true false)
  (set `self.IsEnabled?` true))

(event `/Game/Core/Blueprints/Interaction/BPI_Interaction.InteractWithOject`
  (if (`self.IsEnabled?`)
    (`/Engine/EditorBlueprintResources/StandardMacros.DoOnce` false
      (:`Completed`
        (`GameplayStatics.PlaySound2D` "/Game/Sounds/pagegrab.pagegrab" 1.0 1.0 0.0 null null)
        (bind _returnvalue (`GameplayStatics.GetActorOfClass` "/Game/Characters/Player/Blueprints/BP_Player.BP_Player_C"))
        (set `/Game/Characters/Player/Blueprints/BP_Player.PagesCollected` (+ 1 (`/Game/Characters/Player/Blueprints/BP_Player.PagesCollected` _returnvalue)) _returnvalue)
        (`/Game/Characters/Player/Blueprints/BP_Player.PageUpdate` _returnvalue)
        (`self.K2_DestroyActor`)))))

(event `self.Box.OnComponentBeginOverlap`
  (params (OverlappedComponent :type "PrimitiveComponent Object Reference") (OtherActor :type "Actor Object Reference") (OtherComp :type "PrimitiveComponent Object Reference") (OtherBodyIndex :type Integer) (bFromSweep :type Boolean) (SweepResult :type "HitResult Structure (by ref)"))
  (if (`self.IsEnabled?`)
    (bind _asbp_player (cast `/Game/Characters/Player/Blueprints/BP_Player` OtherActor))
    (bind _output_get (set `self.PlayerInBound` true))
    (if (and _output_get (`/Game/Characters/Player/Blueprints/BP_Player.WeSeePage` _asbp_player))
      (`/Engine/EditorBlueprintResources/StandardMacros.DoOnce` false :!label _label
        (:`Completed`
          (`SceneComponent.SetVisibility` (`/Game/Characters/Player/Blueprints/BP_Player.FlashlightModel` _asbp_player) false false)
          (`SceneComponent.SetVisibility` (`/Game/Characters/Player/Blueprints/BP_Player.Main` _asbp_player) false false)
          (`SceneComponent.SetVisibility` (`self.Flashlight`) true false)
          (`|ExecutionSequence`
            (:`then_1`
              (goto _label_2 :!via `Reset`))))))))

(event `self.Box.OnComponentEndOverlap`
  (params (OverlappedComponent :type "PrimitiveComponent Object Reference") (OtherActor :type "Actor Object Reference") (OtherComp :type "PrimitiveComponent Object Reference") (OtherBodyIndex :type Integer))
  (if (`self.IsEnabled?`)
    (bind _asbp_player (cast `/Game/Characters/Player/Blueprints/BP_Player` OtherActor))
    (set `self.PlayerInBound` false)
    (`/Engine/EditorBlueprintResources/StandardMacros.DoOnce` false :!label _label_2
      (:`Completed`
        (`SceneComponent.SetVisibility` (`/Game/Characters/Player/Blueprints/BP_Player.FlashlightModel` _asbp_player) true false)
        (`SceneComponent.SetVisibility` (`/Game/Characters/Player/Blueprints/BP_Player.Main` _asbp_player) true false)
        (`SceneComponent.SetVisibility` (`self.Flashlight`) false false)
        (goto _label :!via `Reset`)))))

(fn `UserConstructionScript`)