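; Thunder effect Blueprint that plays recurring lightning flashes and thunder sound at random intervals of roughly 20 to 30 seconds.
; Tick enters a DoOnce that starts each delayed cycle, briefly setting IsThunder so Tick shows the DirectionalLight and randomizes its intensity for flicker.
; After the flash window it spawns the 2D thunder cue, hides the light and resets both DoOnce gates to repeat.
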(event `Reset Thunder`
  (goto _label :!via `Reset`))

(event `Reset ThunderFX`
  (goto _label_2 :!via `Reset`))

(event `self.ReceiveTick`
  (params (DeltaSeconds :type "Float (single-precision)"))
  (`|ExecutionSequence`
    (:`then_0`
      (`/Engine/EditorBlueprintResources/StandardMacros.DoOnce` false :!label _label
        (:`Completed`
          (`KismetSystemLibrary.Delay` (`KismetMathLibrary.RandomFloatInRange` 20.1 30.0))
          (set `self.IsThunder` true)
          (`KismetSystemLibrary.Delay` 0.5)
          (`/Engine/EditorBlueprintResources/StandardMacros.DoOnce` false :!label _label_2
            (:`Completed`
              (`|ExecutionSequence`
                (:`then_0`
                  (`GameplayStatics.SpawnSound2D` "/Game/Sounds/Cue/Thunder_CUE.Thunder_CUE" 1.0 1.0 0.0 null)
                  (`self.Reset Thunder`))
                (:`then_1`
                  (set `self.IsThunder` false)
                  (`SceneComponent.SetVisibility` (`self.DirectionalLight`) false false)
                  (`self.Reset ThunderFX`))))))))
    (:`then_1`
      (if (`self.IsThunder`)
        (`SceneComponent.SetVisibility` (`self.DirectionalLight`) true false)
        (`KismetSystemLibrary.Delay` 0.05)
        (`LightComponent.SetIntensity` (`self.DirectionalLight`) (`KismetMathLibrary.RandomFloatInRange` 0.01 2.0))))))

(event `self.ReceiveBeginPlay`
  (`SceneComponent.SetVisibility` (`self.DirectionalLight`) false false)
  (set `self.IsThunder` false))

(fn `UserConstructionScript`)