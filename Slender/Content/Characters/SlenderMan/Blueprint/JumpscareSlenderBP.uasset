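; JumpscareSlenderBP is the Slender Man jumpscare sequence that ends by returning the player to the main menu.
; ScareTime fires once, looping an animation on four tendrils while the Scale timeline drives their world scale.
; The first timeline update plays a distorted static sound and starts an endless Delay loop that randomly flickers the spotlight's intensity.
; In parallel, a timed delay opens LVL_MainMenu.
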(event `ScareTime`
  (`/Engine/EditorBlueprintResources/StandardMacros.DoOnce` false
    (:`Completed`
      (`SkeletalMeshComponent.PlayAnimation` (`self.Tendril2`) "/Game/Characters/SlenderMan/Model/Tendril_with_animation_test_Anim.Tendril_with_animation_test_Anim" true)
      (`SkeletalMeshComponent.PlayAnimation` (`self.Tendril3`) "/Game/Characters/SlenderMan/Model/Tendril_with_animation_test_Anim.Tendril_with_animation_test_Anim" true)
      (`SkeletalMeshComponent.PlayAnimation` (`self.Tendril4`) "/Game/Characters/SlenderMan/Model/Tendril_with_animation_test_Anim.Tendril_with_animation_test_Anim" true)
      (`SkeletalMeshComponent.PlayAnimation` (`self.Tendril1`) "/Game/Characters/SlenderMan/Model/Tendril_with_animation_test_Anim.Tendril_with_animation_test_Anim" true)
      (bind (_direction _scaletendril) (`Timeline|Scale`)
        (:`Update`
          (`SceneComponent.SetWorldScale3D` (`self.Tendril1`) (`KismetMathLibrary.MakeVector` _scaletendril _scaletendril _scaletendril))
          (`SceneComponent.SetWorldScale3D` (`self.Tendril4`) (`KismetMathLibrary.MakeVector` _scaletendril _scaletendril _scaletendril))
          (`SceneComponent.SetWorldScale3D` (`self.Tendril3`) (`KismetMathLibrary.MakeVector` _scaletendril _scaletendril _scaletendril))
          (`SceneComponent.SetWorldScale3D` (`self.Tendril2`) (`KismetMathLibrary.MakeVector` _scaletendril _scaletendril _scaletendril))
          (`/Engine/EditorBlueprintResources/StandardMacros.DoOnce` false
            (:`Completed`
              (`GameplayStatics.PlaySound2D` "/Game/Characters/SlenderMan/Sounds/DISTOTED_STATIC__2__Cue.DISTOTED_STATIC__2__Cue" 1.0 1.0 0.0 null null)
              (`|ExecutionSequence`
                (:`then_0`
                  (`LightComponent.SetIntensity` (`self.SpotLight`) (`KismetMathLibrary.RandomFloatInRange` 0.0 3000.0) :!label _label)
                  (`KismetSystemLibrary.Delay` 0.05)
                  (goto _label))
                (:`then_1`
                  (`KismetSystemLibrary.Delay` 12.0)
                  (`GameplayStatics.OpenLevel` "LVL_MainMenu"))))))))))

(fn `UserConstructionScript`)