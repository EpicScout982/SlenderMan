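; SlenderMan enemy character that pursues PlayerBP, halting and calling SlendySee on the player when recently rendered.
; Tick runs this only while CanMove is false, and BeginPlay sets it true after a short delay.
; Distance hides the mesh when far and reveals it when near unless IsInSight, while collected pages raise walk speed.
; Box overlap while visible sets Scare, whose only check is unwired.
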(event `self.ReceiveBeginPlay`
  (`KismetSystemLibrary.Delay` 2.0)
  (set `self.CanMove?` true))

(event `self.ReceiveTick`
  (params (DeltaSeconds :type "Float (single-precision)"))
  (if (not (`self.CanMove?`))
    (bind _returnvalue (`GameplayStatics.GetActorOfClass` "/Game/Blueprints/Player/PlayerBP.PlayerBP_C"))
    (`|ExecutionSequence`
      (:`then_0`
        (if (`self.WasRecentlyRendered` 0.0)
          (`MovementComponent.StopMovementImmediately` (`self.CharacterMovement`))
          (`/Game/Blueprints/Player/PlayerBP.SlendySee` _returnvalue)
          (else
            (`|AIMoveTo` self (0.0 0.0 0.0) _returnvalue))))
      (:`then_1`
        (bind _returnvalue_2 (`self.GetDistanceTo` _returnvalue))
        (if (>= _returnvalue_2 3000.0)
          (set `self.Visible?` false)
          (`SceneComponent.SetVisibility` (`self.Mesh`) false false)
          (elif (< _returnvalue_2 1700.0)
            (if (`self.IsInSight?`)
              (`MovementComponent.StopMovementImmediately` (`self.CharacterMovement`))
              (else
                (set `self.Visible?` true)
                (`SceneComponent.SetVisibility` (`self.Mesh`) true false)))))))))

(event `SlenderPageUpdate`
  (bind _charactermovement (`self.CharacterMovement`))
  (switch `int` (`/Game/Blueprints/Player/PlayerBP.PagesCollected` (stale `self.ReceiveTick` _returnvalue))
    (:`1`
      (set `CharacterMovementComponent.MaxWalkSpeed` 325.0 _charactermovement))
    (:`2`
      (set `CharacterMovementComponent.MaxWalkSpeed` 350.0 _charactermovement))
    (:`3`
      (set `CharacterMovementComponent.MaxWalkSpeed` 375.0 _charactermovement))
    (:`4`
      (set `CharacterMovementComponent.MaxWalkSpeed` 400.0 _charactermovement))
    (:`5`
      (set `CharacterMovementComponent.MaxWalkSpeed` 425.0 _charactermovement))
    (:`6`
      (set `CharacterMovementComponent.MaxWalkSpeed` 450.0 _charactermovement))
    (:`7`
      (set `CharacterMovementComponent.MaxWalkSpeed` 475.0 _charactermovement))))

(event `self.Box.OnComponentBeginOverlap`
  (params (OverlappedComponent :type "PrimitiveComponent Object Reference") (OtherActor :type "Actor Object Reference") (OtherComp :type "PrimitiveComponent Object Reference") (OtherBodyIndex :type Integer) (bFromSweep :type Boolean) (SweepResult :type "HitResult Structure (by ref)"))
  (if (`self.Visible?`)
    (set `self.Scare` true)))

(fn `UserConstructionScript`)