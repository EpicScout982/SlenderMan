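; First-person player character for a Slender Man horror game, with flashlight, zoom, stamina-limited sprint, pause menu and trace-based interface interaction.
; Pawn sensing of SlenderMan within range drives a timeline that blends white-noise static, layers static audio and triggers his scare at full blend.
; Page updates notify SlenderMan, teleporting and activating him on the first page.
; Looping timers run stamina and surface-based footsteps, while Tick handles headbob, static and exhaustion slowdown.
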(event `InputAxis|MoveForward` :overrideparent false
  (params (AxisValue :type "Float (single-precision)"))
  ;[1 1 1] PlayerMovement
  (`self.AddMovementInput` (`KismetMathLibrary.GetForwardVector` (`KismetMathLibrary.MakeRotator` 0.0 0.0 (.yaw (`self.GetControlRotation`)))) AxisValue))

(event `InputAxis|MoveRight` :overrideparent false
  (params (AxisValue :type "Float (single-precision)"))
  ;[1 1 1] PlayerMovement
  (`self.AddMovementInput` (`KismetMathLibrary.GetRightVector` (`KismetMathLibrary.MakeRotator` 0.0 0.0 (.yaw (`self.GetControlRotation`)))) AxisValue))

(event `PageUpdate`
  ;[1 1 1] Page Update
  (`|ExecutionSequence`
    (:`then_0`
      (if (== (`self.PagesCollected`) 1)
        (bind _returnvalue (`GameplayStatics.GetActorOfClass` "/Game/Characters/SlenderMan/Blueprint/SlenderManBP.SlenderManBP_C"))
        (`self.K2_TeleportTo` :`self` _returnvalue :`DestLocation` (3590.0 4440.0 112.216278))
        (`KismetSystemLibrary.Delay` 0.2)
        (set `/Game/Characters/SlenderMan/Blueprint/SlenderManBP.CanMove?` true _returnvalue)))
    (:`then_1`
      (`/Game/Characters/SlenderMan/Blueprint/SlenderManBP.SlenderPageUpdate` _returnvalue))))

(event `Key|RightMouseButton`
  (params (Key :type "Key Structure"))
  (bind _main (`self.Main`))
  ;[1 1 1] Flashlight
  (:`Pressed`
    (`/Engine/EditorBlueprintResources/StandardMacros.FlipFlop`
      (:`A`
        (`GameplayStatics.PlaySound2D` "/Game/Sounds/FlashLightClicker.FlashLightClicker" 1.0 1.0 0.0 null null)
        (`KismetSystemLibrary.Delay` 0.1)
        (`SceneComponent.SetVisibility` _main false false)
        (`SceneComponent.SetVisibility` (`self.FakeLightCone`) false false)
        (set `self.IsFlashLightOn?` false))
      (:`B`
        (`GameplayStatics.PlaySound2D` "/Game/Sounds/FlashLightClicker.FlashLightClicker" 1.0 1.0 0.0 null null :!label _label)
        (`KismetSystemLibrary.Delay` 0.1)
        (`SceneComponent.SetVisibility` _main true false)
        (`SceneComponent.SetVisibility` (`self.FakeLightCone`) true false)
        (set `self.IsFlashLightOn?` true)))))

(event `self.PawnSensing.OnSeePawn`
  (params (Pawn :type "Pawn Object Reference"))
  ;[1 1 1] PawnSensing
  (bind _asslender_man_bp (cast `/Game/Characters/SlenderMan/Blueprint/SlenderManBP` Pawn))
  (set `/Game/Characters/SlenderMan/Blueprint/SlenderManBP.IsInSight?` true _asslender_man_bp)
  (`|ExecutionSequence`
    (:`then_0`
      (bind _returnvalue (`self.GetDistanceTo` _asslender_man_bp))
      (if (< _returnvalue 2000.0)
        (set `self.StaticEnable` true)
        (if (and (<= _returnvalue 600.0) false)
          (`/Engine/EditorBlueprintResources/StandardMacros.DoOnce` false :!label _label_2
            (:`Completed`
              (`GameplayStatics.PlaySound2D` "/Game/Characters/SlenderMan/Blueprint/SlenderApearRemaster.SlenderApearRemaster" 1.0 1.0 0.0 null null)
              (`KismetSystemLibrary.Delay` 30.0)
              (goto _label_2 :!via `Reset`))))
        (else
          (set `self.StaticEnable` false :!label _label_3))))
    (:`then_1`
      (`KismetSystemLibrary.Delay` 3.0)
      (set `/Game/Characters/SlenderMan/Blueprint/SlenderManBP.IsInSight?` false _asslender_man_bp)
      (goto _label_3))))

(event `InputAxis|Turn` :overrideparent false
  (params (AxisValue :type "Float (single-precision)"))
  ;[1 1 1] Mouse Looking
  (`self.AddControllerYawInput` AxisValue))

(event `self.ReceiveBeginPlay`
  (bind _returnvalue (`GameplayStatics.GetPlayerCameraManager` 0))
  ;[1 1 1] StartUp
  (`|ExecutionSequence`
    (:`then_0`
      (`SceneComponent.SetVisibility` (`self.Main`) true false)
      (`SceneComponent.SetVisibility` (`self.FakeLightCone`) true false)
      (bind _returnvalue_2 (`|CreateWidget` "/Game/GUI/Hud/Blueprints/BP_Hud.BP_Hud_C"))
      (`UserWidget.AddToViewport` _returnvalue_2 0)
      (set `self.Sanity` 1.0))
    (:`then_1`
      ;[1 1 1] Flashlight
      (`KismetSystemLibrary.Delay` 2.5)
      (goto _label))
    (:`then_2`
      (set `PlayerCameraManager.ViewPitchMin` -30.0 _returnvalue)
      (set `PlayerCameraManager.ViewPitchMax` 60.0 _returnvalue))
    (:`then_3`
      (`self.Footstep`))
    (:`then_4`
      (`self.StaminaUpdate`))))

(event `self.ReceiveTick`
  (params (DeltaSeconds :type "Float (single-precision)"))
  ;[1 1 1] Event Tick
  (`|ExecutionSequence`
    (:`then_0`
      (`self.Headbob`))
    (:`then_1`
      (`self.StaticCommit`))
    (:`then_2`
      (`self.ClearStamina`))))

(event `InputAxis|LookUp` :overrideparent false
  (params (AxisValue :type "Float (single-precision)"))
  ;[1 1 1] Mouse Looking
  (`self.AddControllerPitchInput` AxisValue))

(event `self.Box.OnComponentBeginOverlap`
  (params (OverlappedComponent :type "PrimitiveComponent Object Reference") (OtherActor :type "Actor Object Reference") (OtherComp :type "PrimitiveComponent Object Reference") (OtherBodyIndex :type Integer) (bFromSweep :type Boolean) (SweepResult :type "HitResult Structure (by ref)"))
  ;[1 1 1] Page See
  (cast `/Game/Core/Blueprints/Interaction/BP_Page` OtherActor)
  (set `self.WeSeePage` true))

(event `Key|Escape`
  (params (Key :type "Key Structure"))
  ;[1 1 1] Pause Menu
  (:`Pressed`
    (bind _returnvalue (`|CreateWidget` "/Game/GUI/PauseMenu/Blueprint/PauseScreen_WIDGET.PauseScreen_WIDGET_C" :!label _label_4))
    (`UserWidget.AddToViewport` _returnvalue 0)
    (`WidgetBlueprintLibrary.SetInputMode_UIOnlyEx` (`GameplayStatics.GetPlayerController` 0) _returnvalue)))

(event `RunCheck`
  (bind (_returnvalue_roll _returnvalue_pitch _returnvalue_yaw) (`KismetMathLibrary.BreakRotator` (`SceneComponent.K2_GetComponentRotation` (`self.Camera`))))
  ;[1 1 1] Running
  (bind (_direction _fl) (`Timeline|FlashlightRunning` :!label _label_5)
    (:`Update`
      (`SceneComponent.K2_SetWorldRotation` (`self.FlashlightSpring`) (`KismetMathLibrary.MakeRotator` 0.0 (+ _fl _returnvalue_pitch) _returnvalue_yaw) false false))))

(event `Key|LeftMouseButton`
  (params (Key :type "Key Structure"))
  ;[1 1 1] 3CameraZoom
  (:`Pressed`
    (if (not (`self.IsRunning?`))
      (set `self.IsZoom?` true)
      (`AudioComponent.Play` (`self.CamZoomIn`) 0.0)
      (`AudioComponent.Stop` (`self.CamZoomOut`))
      (bind (_direction _zoom) (`Timeline|Zoom` :!label _label_6)
        (:`Update`
          (`CameraComponent.SetFieldOfView` (`self.Camera`) _zoom))
        (:`Finished`
          (`AudioComponent.Stop` (`self.CamZoomOut`))
          (`AudioComponent.Stop` (`self.CamZoomIn`))))))
  (:`Released`
    (if (not (`self.IsRunning?`))
      (set `self.IsZoom?` false)
      (`AudioComponent.Play` (`self.CamZoomOut`) 0.0)
      (`AudioComponent.Stop` (`self.CamZoomIn`))
      (goto _label_6 :!via `Reverse`))))

(event `Key|LeftShift`
  (params (Key :type "Key Structure"))
  ;[1 1 1] Running
  (:`Pressed`
    (if (`self.IsZoom?`)
      _
      (elif (not (`self.Exausted`))
        (set `self.IsRunning?` true)
        (set `CharacterMovementComponent.MaxWalkSpeed` 400.0 (`self.CharacterMovement`))
        (`|ExecutionSequence`
          (:`then_0`
            (goto _label_5 :!via `PlayFromStart`))
          (:`then_1`
            (bind (_direction _fov) (`Timeline|RunningFOV` :!via `PlayFromStart`)
              (:`Update`
                (`CameraComponent.SetFieldOfView` (`self.Camera`) _fov))))))))
  (:`Released`
    (if (not (`self.IsZoom?`))
      (set `self.IsRunning?` false)
      (set `CharacterMovementComponent.MaxWalkSpeed` 200.0 (`self.CharacterMovement`))
      (if (not (< (`self.StaminaValue`) 20.0))
        (`|ExecutionSequence`
          (:`then_0`
            (goto _label_5 :!via `Reverse`))
          (:`then_1`
            (bind (_direction_2 _fov_2) (`Timeline|FOVReset` :!via `PlayFromStart` :!label _label_7)
              (:`Update`
                (`CameraComponent.SetFieldOfView` (`self.Camera`) _fov_2)))))))))

(event `Key|P`
  (params (Key :type "Key Structure"))
  ;[1 1 1] Pause Menu
  (:`Pressed`
    (goto _label_4)))

(event `self.Box.OnComponentEndOverlap`
  (params (OverlappedComponent :type "PrimitiveComponent Object Reference") (OtherActor :type "Actor Object Reference") (OtherComp :type "PrimitiveComponent Object Reference") (OtherBodyIndex :type Integer))
  ;[1 1 1] Page See 2
  (cast `/Game/Core/Blueprints/Interaction/BP_Page` OtherActor)
  (set `self.WeSeePage` false))

(event `StaticCommit`
  ;[1 1 1] Static
  (if (`self.StaticEnable`)
    (set `self.WeSeeSlender` true)
    (bind (_direction _static_ _staticsounds) (`Timeline|SlenderStatic` :!label _label_8)
      (:`Update`
        (bind _output_get (set `PostProcessComponent.BlendWeight` _static_ (`self.WhiteNoise`)))
        (`|ExecutionSequence`
          (:`then_0`
            (if (== _output_get 1.0)
              (`/Engine/EditorBlueprintResources/StandardMacros.DoOnce` false
                (:`Completed`
                  (bind _returnvalue (`GameplayStatics.GetActorOfClass` "/Game/Characters/SlenderMan/Blueprint/SlenderManBP.SlenderManBP_C"))
                  (set `/Game/Characters/SlenderMan/Blueprint/SlenderManBP.Scare` true _returnvalue)))))
          (:`then_1`
            (if (<= _staticsounds 0.99)
              (`|ExecutionSequence`
                (:`then_0`
                  (`/Engine/EditorBlueprintResources/StandardMacros.DoOnce` false :!label _label_9
                    (:`Completed`
                      (`AudioComponent.FadeIn` (`self.LightStatic`) 1.0 1.0 0.0 "Linear"))))
                (:`then_1`
                  (if (<= _staticsounds 0.66)
                    (`|ExecutionSequence`
                      (:`then_0`
                        (`/Engine/EditorBlueprintResources/StandardMacros.DoOnce` false :!label _label_10
                          (:`Completed`
                            (`AudioComponent.FadeIn` (`self.MediumStatic`) 1.0 1.0 0.0 "Linear"))))
                      (:`then_1`
                        (if (<= _staticsounds 0.33)
                          (`/Engine/EditorBlueprintResources/StandardMacros.DoOnce` false :!label _label_11
                            (:`Completed`
                              (`AudioComponent.FadeIn` (`self.HeavyStatic`) 1.0 1.0 0.0 "Linear")))
                          (else
                            (`AudioComponent.FadeOut` (`self.HeavyStatic`) 1.0 0.0 "Linear")
                            (goto _label_11 :!via `Reset`)))))
                    (else
                      (`AudioComponent.FadeOut` (`self.MediumStatic`) 1.0 0.0 "Linear")
                      (goto _label_10 :!via `Reset`)))))
              (else
                (`AudioComponent.FadeOut` (`self.LightStatic`) 1.0 0.0 "Linear")
                (goto _label_9 :!via `Reset`)))))))
    (else
      (set `self.WeSeeSlender` false)
      (goto _label_8 :!via `Reverse`))))

(event `ClearStamina`
  (if (< (`self.StaminaValue`) 20.0)
    (`/Engine/EditorBlueprintResources/StandardMacros.DoOnce` false :!label _label_12
      (:`Completed`
        (set `CharacterMovementComponent.MaxWalkSpeed` 200.0 (`self.CharacterMovement`))
        (goto _label_7 :!via `PlayFromStart`)))
    (else
      (set `self.Exausted` false)
      (goto _label_12 :!via `Reset`))))

(event `InputAction|Interact`
  (params (Key :type "Key Structure"))
  ;[1 1 1] Interaction System
  (:`Pressed`
    (`self.F_Interaction`)))

(event `Headbob`
  ;[1 1 1] Headbob
  (`self.F_Headbob`))

(event `StaminaUpdate`
  ;[1 1 1] Stamina
  (`KismetSystemLibrary.K2_SetTimerDelegate` (delegate `Stamina`) 0.1 true))

(event `Stamina`
  ;[1 1 1] Stamina
  (`self.F_Stamina`))

(event `Footstep`
  ;[1 1 1] Footsteps
  (`KismetSystemLibrary.K2_SetTimerDelegate` (delegate `Footsteps`) 0.5 true))

(event `Footsteps`
  ;[1 1 1] Footsteps
  (`self.F_PhyMatSoundSFX`))

(fn `F_Headbob`
  (bind _returnvalue (`GameplayStatics.GetPlayerCameraManager` 0))
  (bind _returnvalue_2 (`KismetMathLibrary.VSize` (`self.GetVelocity`)))
  (if (> _returnvalue_2 0.0)
    (if (< _returnvalue_2 300.0)
      (`MatineeCameraShake.StartMatineeCameraShake` _returnvalue "/Game/Characters/Player/Blueprints/HeadBobbing/Player_WalkBob.Player_WalkBob_C")
      (else
        (`MatineeCameraShake.StartMatineeCameraShake` _returnvalue "/Game/Characters/Player/Blueprints/HeadBobbing/Player_RunBob.Player_RunBob_C")))
    (else
      (`MatineeCameraShake.StartMatineeCameraShake` _returnvalue "/Game/Characters/Player/Blueprints/HeadBobbing/Player_IdeBob.Player_IdeBob_C"))))

(fn `F_Interaction`
  (bind _camera (`self.Camera`))
  (bind _returnvalue (`SceneComponent.K2_GetComponentLocation` _camera))
  (bind _outhit (`KismetSystemLibrary.LineTraceSingleForObjects` _returnvalue (+ _returnvalue (* (`SceneComponent.GetForwardVector` _camera) 120.0)) (`|MakeArray` "ObjectTypeQuery1" "ObjectTypeQuery1" "ObjectTypeQuery7" :!type "EObjectTypeQuery Enum")))
  (bind (_bblockinghit _binitialoverlap _time _distance _location _impactpoint _normal _impactnormal _physmat _hitactor) (`GameplayStatics.BreakHitResult` _outhit))
  (if _bblockinghit
    (if (`KismetSystemLibrary.DoesImplementInterface` _hitactor "/Game/Core/Blueprints/Interaction/BPI_Interaction.BPI_Interaction_C")
      (message `/Game/Core/Blueprints/Interaction/BPI_Interaction.InteractWithOject` _hitactor))))

(fn `F_PhyMatSoundSFX`
  (bind _returnvalue (`self.K2_GetActorLocation`))
  (bind _returnvalue_2 (`SceneComponent.K2_GetComponentLocation` (`self.Camera`)))
  (if (> (`KismetMathLibrary.VSize` (`self.GetVelocity`)) 0.0)
    (bind (_outhit _returnvalue_3) (`KismetSystemLibrary.LineTraceSingle` _returnvalue_2 (- _returnvalue_2 (0.0 0.0 300.0)) "TraceTypeQuery1"))
    (if _returnvalue_3
      (switch `EPhysicalSurface` (`PhysicalMaterial.SurfaceType` (`.PhysMat` (`GameplayStatics.BreakHitResult` _outhit)))
        (:`SurfaceType1`
          (`GameplayStatics.PlaySoundAtLocation` "/Game/Sounds/Footsteps/Dirt/Foot_Dirt1_LightWalk01_Cue.Foot_Dirt1_LightWalk01_Cue" _returnvalue (struct) 1.0 1.0 0.0 null null null))
        (:`SurfaceType2`
          (`GameplayStatics.PlaySoundAtLocation` "/Game/Sounds/Footsteps/Grass/step1_Cue.step1_Cue" _returnvalue (struct) 1.0 1.0 0.0 null null null))
        (:`SurfaceType3`
          (`GameplayStatics.PlaySoundAtLocation` "/Game/Sounds/Footsteps/Inside/tilestep2_Cue.tilestep2_Cue" _returnvalue (struct) 1.0 1.0 0.0 null null null))))))

(fn `F_Stamina`
  (if (> (`KismetMathLibrary.VSize` (`self.GetVelocity`)) 390.0)
    (bind _output_get (set `self.StaminaValue` (`KismetMathLibrary.FClamp` (- (`self.StaminaValue`) 1.0) 0.0 100.0)))
    (else
      (bind _output_get_2 (set `self.StaminaValue` (`KismetMathLibrary.FClamp` (+ (`self.StaminaValue`) 0.1) 0.0 100.0))))))

(fn `UserConstructionScript`)