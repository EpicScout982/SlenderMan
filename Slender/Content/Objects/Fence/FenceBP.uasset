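; Fence Blueprint that tiles fence meshes into runs along the X and Y axes for level building.
; The construction script runs two loops, driven by TilingAmountX and TilingAmountY, adding a scaled static mesh at fixed spacing from the Fence component's world location.
; Pieces use manual attachment and copy the actor's rotation, but their offsets follow world axes rather than rotating with the actor.
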(fn `UserConstructionScript`
  (bind (_returnvalue_x _returnvalue_y _returnvalue_z) (`KismetMathLibrary.BreakVector` (`SceneComponent.K2_GetComponentLocation` (`self.Fence`))))
  (bind (_returnvalue_x_2 _returnvalue_y_2 _returnvalue_z_2) (`KismetMathLibrary.BreakVector` (`SceneComponent.K2_GetComponentLocation` (`self.Fence`))))
  (`|ExecutionSequence`
    (:`then_0`
      (for _index (range (+ (`self.TilingAmount Y`) 1))
        (`AddComponent|NODE_AddStaticMeshComponent-0` :`bManualAttachment` true :`RelativeTransform` (`KismetMathLibrary.MakeTransform` (`KismetMathLibrary.MakeVector` _returnvalue_x (+ _returnvalue_y (`KismetMathLibrary.Conv_IntToDouble` (* _index 195))) _returnvalue_z) (`self.K2_GetActorRotation`) (0.0425 0.0425 0.0425)))))
    (:`then_1`
      (for _index_2 (range (+ (`self.TilingAmount X`) 1))
        (`AddComponent|NODE_AddStaticMeshComponent-2` :`bManualAttachment` true :`RelativeTransform` (`KismetMathLibrary.MakeTransform` (`KismetMathLibrary.MakeVector` (+ _returnvalue_x_2 (`KismetMathLibrary.Conv_IntToDouble` (* _index_2 195))) _returnvalue_y_2 _returnvalue_z_2) (`self.K2_GetActorRotation`) (0.0425 0.0425 0.0425)))))))