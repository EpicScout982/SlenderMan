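; BP_Crickets is an ambient sound Blueprint that plays cricket, owl and distant dog sounds at random intervals.
; Tick drives three independent loops through a Sequence, each using a DoOnce gate that waits a random Delay, plays its sound and resets.
; Crickets repeat every few seconds, while the owl and dog are much rarer.
; All sounds are spawned as non-positional 2D audio.
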(event `self.ReceiveTick`
  (params (DeltaSeconds :type "Float (single-precision)"))
  (`|ExecutionSequence`
    (:`then_0`
      (`/Engine/EditorBlueprintResources/StandardMacros.DoOnce` false :!label _label
        (:`Completed`
          (`KismetSystemLibrary.Delay` (`KismetMathLibrary.RandomFloatInRange` 1.0 3.0))
          (`GameplayStatics.SpawnSound2D` "/Game/Crickets.Crickets" 1.0 1.0 0.0 null)
          (goto _label :!via `Reset`))))
    (:`then_1`
      (`/Engine/EditorBlueprintResources/StandardMacros.DoOnce` false :!label _label_2
        (:`Completed`
          (`KismetSystemLibrary.Delay` (`KismetMathLibrary.RandomFloatInRange` 10.0 60.0))
          (`GameplayStatics.SpawnSound2D` "/Game/owl.owl" 1.0 1.0 0.0 null)
          (goto _label_2 :!via `Reset`))))
    (:`then_2`
      (`/Engine/EditorBlueprintResources/StandardMacros.DoOnce` false :!label _label_3
        (:`Completed`
          (`KismetSystemLibrary.Delay` (`KismetMathLibrary.RandomFloatInRange` 30.0 120.0))
          (`GameplayStatics.SpawnSound2D` "/Game/dog_distant_agitated.dog_distant_agitated" 1.0 1.0 0.0 null)
          (goto _label_3 :!via `Reset`))))))

(fn `UserConstructionScript`)