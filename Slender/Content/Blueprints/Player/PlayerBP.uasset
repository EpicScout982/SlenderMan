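; First-person player character Blueprint with walking, sprinting, mouse look, camera zoom, a toggleable flashlight and a Sanity value.
; Movement drives looping-timer footsteps and landing sounds, while Tick selects idle, walk or run camera shakes by speed.
; Timelines animate zoom FOV and sprint flashlight tilt; Tick raises Sanity with the flashlight on and lowers it when off.
; It also creates HUD and pause widgets, and line-traces from the camera to call BPI_Interaction.
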(event `InputAxis|MoveForward` :overrideparent false
  (params (AxisValue :type "Float (single-precision)"))
  (bind (_returnvalue_x _returnvalue_y _returnvalue_z) (`KismetMathLibrary.BreakVector` (`self.GetVelocity`)))
  ;[1 1 1] Footstep Sounds
  (`self.AddMovementInput` (`KismetMathLibrary.GetForwardVector` (`KismetMathLibrary.MakeRotator` 0.0 0.0 (.yaw (`self.GetControlRotation`)))) AxisValue)
  (if (and (or (> _returnvalue_x 1.0) (< _returnvalue_x -1.0) (> _returnvalue_y 1.0) (< _returnvalue_y -1.0)) (== _returnvalue_z 0.0)) :!label _label
    (`/Engine/EditorBlueprintResources/StandardMacros.DoOnce` false :!label _label_2
      (:`Completed`
        (bind _returnvalue (`KismetSystemLibrary.K2_SetTimerDelegate` (delegate `Play Footstep Sound`) (`self.FootstepInt`) true))))
    (else
      (`KismetSystemLibrary.K2_ClearAndInvalidateTimerHandle` _returnvalue)
      (goto _label_2 :!via `Reset`))))

(event `Play Footstep Sound`
  ;[1 1 1] Footstep Sounds
  (`GameplayStatics.PlaySoundAtLocation` "/Game/Sounds/Cue/Footstep_CUE.Footstep_CUE" (- (`self.K2_GetActorLocation`) (0.0 0.0 44.0)) (struct) 1.0 1.0 0.0 null null null))

(event `InputAxis|MoveRight` :overrideparent false
  (params (AxisValue :type "Float (single-precision)"))
  ;[1 1 1] Footstep Sounds
  (`self.AddMovementInput` (`KismetMathLibrary.GetRightVector` (`KismetMathLibrary.MakeRotator` 0.0 0.0 (.yaw (`self.GetControlRotation`)))) AxisValue)
  (goto _label))

(event `self.K2_OnMovementModeChanged`
  (params (PrevMovementMode :type "EMovementMode Enum" :default "MOVE_None") (NewMovementMode :type "EMovementMode Enum" :default "MOVE_None") (PrevCustomMode :type Byte) (NewCustomMode :type Byte))
  ;[1 1 1] Jumping Sound sfx
  (if (and (`|EnumEquality` PrevMovementMode "MOVE_Falling") (`|EnumEquality` NewMovementMode "MOVE_Walking"))
    (`self.Play Footstep Sound`)))

(event `Key|RightMouseButton`
  (params (Key :type "Key Structure"))
  (bind _flashlight (`self.Flashlight`))
  ;[1 1 1] Flashlight
  (:`Pressed`
    (`/Engine/EditorBlueprintResources/StandardMacros.FlipFlop`
      (:`A`
        (`GameplayStatics.PlaySound2D` "/Game/Sounds/flashclick.flashclick" 1.0 1.0 0.0 null null)
        (`KismetSystemLibrary.Delay` 0.1)
        (`SceneComponent.SetVisibility` _flashlight false false)
        (set `self.IsFlashLightOn?` false)
        (`self.Reset  Max`)
        (`self.Reset Min`))
      (:`B`
        (`GameplayStatics.PlaySound2D` "/Game/Sounds/flashclick.flashclick" 1.0 1.0 0.0 null null :!label _label_3)
        (`KismetSystemLibrary.Delay` 0.1)
        (`SceneComponent.SetVisibility` _flashlight true false)
        (set `self.IsFlashLightOn?` true)
        (`self.Reset  Max`)
        (`self.Reset Min`)))))

(event `self.ReceiveBeginPlay`
  ;[1 1 1] StartUp
  (`|ExecutionSequence`
    (:`then_0`
      (`SceneComponent.SetVisibility` (`self.Flashlight`) true false)
      (bind _returnvalue (`|CreateWidget` "/Game/Blueprints/Hud_WIDGET1.Hud_WIDGET1_C"))
      (`UserWidget.AddToViewport` _returnvalue 0)
      (set `self.Sanity` 1.0))
    (:`then_1`
      ;[1 1 1] Flashlight
      (`KismetSystemLibrary.Delay` 2.5)
      (goto _label_3))))

(event `Key|P`
  (params (Key :type "Key Structure"))
  ;[1 1 1] PauseMenu
  (:`Pressed`
    (`GameplayStatics.SpawnSound2D` "/Game/Sounds/blip.blip" 1.0 1.0 0.0 null :!label _label_4)
    (bind _returnvalue (`|CreateWidget` "/Game/PauseScreen/PauseScreen_WIDGET.PauseScreen_WIDGET_C"))
    (`UserWidget.AddToViewport` _returnvalue 0)))

(event `Key|LeftMouseButton`
  (params (Key :type "Key Structure"))
  (:`Pressed`
    (`AudioComponent.Play` (`self.CamZoomIn`) 0.0)
    (`AudioComponent.Stop` (`self.CamZoomOut`))
    (bind (_direction _zoom) (`Timeline|Zoom` :!label _label_5)
      (:`Update`
        (`CameraComponent.SetFieldOfView` (`self.Camera`) _zoom))
      (:`Finished`
        (`AudioComponent.Stop` (`self.CamZoomOut`))
        (`AudioComponent.Stop` (`self.CamZoomIn`)))))
  (:`Released`
    (`AudioComponent.Play` (`self.CamZoomOut`) 0.0)
    (`AudioComponent.Stop` (`self.CamZoomIn`))
    (goto _label_5 :!via `Reverse`)))

(event `Key|Escape`
  (params (Key :type "Key Structure"))
  ;[1 1 1] PauseMenu
  (:`Pressed`
    (goto _label_4)))

(event `InputAxis|Turn` :overrideparent false
  (params (AxisValue :type "Float (single-precision)"))
  ;[1 1 1] Mouse Looking
  (`self.AddControllerYawInput` AxisValue))

(event `RunCheck`
  (bind (_returnvalue_roll _returnvalue_pitch _returnvalue_yaw) (`KismetMathLibrary.BreakRotator` (`SceneComponent.K2_GetComponentRotation` (`self.Camera`))))
  ;[1 1 1] Flashlight Move Down
  (if true :!label _label_6
    (bind (_direction _fl) (`Timeline|FlashlightRunning` :!label _label_7)
      (:`Update`
        (`SceneComponent.K2_SetWorldRotation` (`self.FlashlightSpring`) (`KismetMathLibrary.MakeRotator` 0.0 (+ _fl _returnvalue_pitch) _returnvalue_yaw) false false)))))

(event `InputAxis|LookUp` :overrideparent false
  (params (AxisValue :type "Float (single-precision)"))
  ;[1 1 1] Mouse Looking
  (`self.AddControllerPitchInput` AxisValue))

(event `Key|LeftShift`
  (params (Key :type "Key Structure"))
  (bind _charactermovement (`self.CharacterMovement`))
  ;[1 1 1] Flashlight Move Down
  (:`Pressed`
    (set `self.IsRunning?` true)
    (set `CharacterMovementComponent.MaxWalkSpeed` 400.0 _charactermovement)
    (goto _label_6))
  (:`Released`
    (set `self.IsRunning?` false)
    (set `CharacterMovementComponent.MaxWalkSpeed` 200.0 _charactermovement)
    (goto _label_7 :!via `Reverse`)))

(event `Reset  Max`
  ;[1 1 1] Sanity Hell
  (goto _label_8 :!via `Reset`))

(event `Reset Min`
  ;[1 1 1] Sanity Hell
  (goto _label_9 :!via `Reset`))

(event `self.ReceiveTick`
  (params (DeltaSeconds :type "Float (single-precision)"))
  (`|ExecutionSequence`
    (:`then_0`
      ;[1 1 1] Sanity Hell
      (if (> (`self.Sanity`) 100.0)
        (`/Engine/EditorBlueprintResources/StandardMacros.DoOnce` false :!label _label_8
          (:`Completed`
            (set `self.Sanity` 100.0)))
        (elif (< (`self.Sanity`) 0.0)
          (`/Engine/EditorBlueprintResources/StandardMacros.DoOnce` false :!label _label_9
            (:`Completed`
              (set `self.Sanity` 0.0)))
          (else
            (`KismetSystemLibrary.Delay` 0.1)
            (if (`self.IsFlashLightOn?`)
              (set `self.Sanity` (+ (`self.Sanity`) 0.1))
              (else
                (set `self.Sanity` (- (`self.Sanity`) 0.05))))))))
    (:`then_1`
      (`self.IdleHeadBob`)
      (`self.Headbob`))))

(event `InputAction|Interact`
  (params (Key :type "Key Structure"))
  (bind _camera (`self.Camera`))
  (bind _returnvalue (`SceneComponent.K2_GetComponentLocation` _camera))
  (:`Pressed`
    (bind _outhit (`KismetSystemLibrary.LineTraceSingleForObjects` :`Start` _returnvalue :`End` (+ _returnvalue (* (`SceneComponent.GetForwardVector` _camera) 120.0)) :`ObjectTypes` (`|MakeArray` "ObjectTypeQuery1" "ObjectTypeQuery1" "ObjectTypeQuery7" :!type "EObjectTypeQuery Enum") :`DrawDebugType` "ForDuration"))
    (bind (_bblockinghit _binitialoverlap _time _distance _location _impactpoint _normal _impactnormal _physmat _hitactor) (`GameplayStatics.BreakHitResult` _outhit))
    (if _bblockinghit
      (if (`KismetSystemLibrary.DoesImplementInterface` _hitactor "/Game/Blueprints/Player/BPI_Interaction.BPI_Interaction_C")
        (message `/Game/Blueprints/Player/BPI_Interaction.InteractWithOject` _hitactor)))))

(event `IdleHeadBob`)

(event `Headbob`
  (bind _returnvalue (`GameplayStatics.GetPlayerCameraManager` 0))
  (bind _returnvalue_2 (`KismetMathLibrary.VSize` (`self.GetVelocity`)))
  (if (and (> _returnvalue_2 0.0) (`self.CanJump`))
    (if (< _returnvalue_2 300.0)
      (`MatineeCameraShake.StartMatineeCameraShake` _returnvalue "/Game/Blueprints/Player/Player_WalkBob.Player_WalkBob_C")
      (else
        (`MatineeCameraShake.StartMatineeCameraShake` _returnvalue "/Game/Blueprints/Player/Player_RunBob.Player_RunBob_C")))
    (else
      (`MatineeCameraShake.StartMatineeCameraShake` _returnvalue "/Game/Blueprints/Player/Player_IdeBOb.Player_IdeBob_C"))))

(event `Hair Red`)

(event `Hair Yellow`)

(event `Hair Blue`)

(fn `UserConstructionScript`)